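; Labyrinth Blueprint that builds a grid of instanced ground cells as the base for a maze, with only the first visiting step implemented.
; The construction script places Row by Col instances spaced by MeshLenght and records a cell struct for each.
; BeginPlay picks a random start cell and recolors it through per-instance custom data.
; Tick marks that current cell visited after a Delay, without advancing to neighbors.
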(event `self.ReceiveBeginPlay`
  (bind _current (`self.Current`))
  (bind _ground (`self.Ground`))
  (set `self.Current` (`KismetMathLibrary.RandomInteger` (`InstancedStaticMeshComponent.GetInstanceCount` (`self.Ground`))))
  ;[1 1 1] Change color of starting cell
  (bind _returnvalue (`PrimitiveComponent.CreateDynamicMaterialInstance` (`self.Ground`) 0 (`self.Material`) "None"))
  (bind _output_get (set `self.L_DynStart` _returnvalue))
  (`MaterialInstanceDynamic.K2_GetScalarParameterValue` _output_get "ColorStart")
  (`InstancedStaticMeshComponent.SetCustomDataValue` _ground _current 0 0.0 false)
  (`InstancedStaticMeshComponent.SetCustomDataValue` _ground _current 1 1.0 false)
  (`InstancedStaticMeshComponent.SetCustomDataValue` _ground _current 2 1.0 false))

(event `self.ReceiveTick`
  (params (DeltaSeconds :type "Float (single-precision)"))
  (`KismetSystemLibrary.Delay` (`self.Duration`))
  ;[1 1 1] Take current cell and set her as visited
  (bind _structout (setmembers `/Game/Labyrinth_Struct` :`StructRef` (`|GetArrayItem` (`self.ArrayStruct`) (`self.Current`)) :`isVisited` true))
  (`KismetArrayLibrary.Array_Set` (`self.ArrayStruct`) (`self.Current`) _structout))

(fn `UserConstructionScript`
  (locals (IndexRow :type Integer) (IndexCol :type Integer) (`Location Y` :type Integer) (`Location X` :type Integer))
  (bind (_returnvalue_min _returnvalue_max) (break `Box` (`StaticMesh.GetBoundingBox` (`self.GroundMesh`))))
  (`PrimitiveComponent.SetMaterial` (`self.Ground`) 0 (`self.Material`))
  (`KismetArrayLibrary.Array_Clear` (`self.ArrayStruct`))
  (`StaticMeshComponent.SetStaticMesh` (`self.Ground`) (`self.GroundMesh`))
  (set `self.Cell Size` (`KismetMathLibrary.FTrunc` (.x (- _returnvalue_max _returnvalue_min))))
  (for _index (range (`self.Row`))
    (set `local.IndexRow` _index)
    (for _index_2 (range (`self.Col`))
      (set `local.IndexCol` _index_2)
      (`InstancedStaticMeshComponent.AddInstance` (`self.Ground`) (`KismetMathLibrary.MakeTransform` (`KismetMathLibrary.MakeVector` (* _index (`self.MeshLenght`)) (* _index_2 (`self.MeshLenght`)))) false)
      (`KismetArrayLibrary.Array_Add` (`self.ArrayStruct`) (make `/Game/Labyrinth_Struct` (`local.IndexRow`) (`local.IndexCol`))))))